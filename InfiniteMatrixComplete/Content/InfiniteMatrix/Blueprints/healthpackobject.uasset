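; Health pack pickup that heals BP_Player on overlap, clamping Health to its valid range, then destroys itself.
; Two components, Sphere and Sphere1, carry identical overlap handlers, so touching either one consumes the whole actor.
; On BeginPlay a coin flip decides whether Sphere shifts by a random local offset, while Sphere1 is left in place.
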(event `self.ReceiveBeginPlay`
  (if (`KismetMathLibrary.RandomBool`)
    (`SceneComponent.K2_AddLocalOffset` (`self.Sphere`) (`KismetMathLibrary.MakeVector` (`KismetMathLibrary.RandomFloatInRange` 100.0 2200.0) (`KismetMathLibrary.RandomFloatInRange` -100.0 100.0) (`KismetMathLibrary.RandomFloatInRange` -430.0 430.0)) false false)))

(event `self.Sphere.OnComponentBeginOverlap`
  (params (OverlappedComponent :type "PrimitiveComponent Object Reference") (OtherActor :type "Actor Object Reference") (OtherComp :type "PrimitiveComponent Object Reference") (OtherBodyIndex :type Integer) (bFromSweep :type Boolean) (SweepResult :type "HitResult Structure (by ref)"))
  (bind _asbp_player (cast `/Game/InfiniteMatrix/Blueprints/BP_Player` OtherActor))
  (set `/Game/InfiniteMatrix/Blueprints/BP_Player.Health` (`KismetMathLibrary.FClamp` (+ (`/Game/InfiniteMatrix/Blueprints/BP_Player.Health` _asbp_player) 20.0) 0.0 100.0) _asbp_player)
  (`self.K2_DestroyActor`))

(event `self.Sphere1.OnComponentBeginOverlap`
  (params (OverlappedComponent :type "PrimitiveComponent Object Reference") (OtherActor :type "Actor Object Reference") (OtherComp :type "PrimitiveComponent Object Reference") (OtherBodyIndex :type Integer) (bFromSweep :type Boolean) (SweepResult :type "HitResult Structure (by ref)"))
  (bind _asbp_player (cast `/Game/InfiniteMatrix/Blueprints/BP_Player` OtherActor))
  (set `/Game/InfiniteMatrix/Blueprints/BP_Player.Health` (`KismetMathLibrary.FClamp` (+ (`/Game/InfiniteMatrix/Blueprints/BP_Player.Health` _asbp_player) 20.0) 0.0 100.0) _asbp_player)
  (`self.K2_DestroyActor`))

(fn `UserConstructionScript`)